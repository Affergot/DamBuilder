(event Custom|PreviewLoop
  (bind _spectator_camera (Variables|Default|GetSpectator%20Camera))
  (bind _scenecomponent (Variables|/Script/Engine.CameraActor|GetSceneComponent _spectator_camera))
  (bind _returnvalue (Transformation|GetWorldTransform _scenecomponent))
  (bind (_outhit _returnvalue_2) (Collision|LineTraceByChannel (.location _returnvalue) (+ (.location _returnvalue) (+ (Math|Vector|GetForwardVector (.rotation _returnvalue)) 7e+02)) "TraceTypeQuery1" false 0 "ForDuration"))
  (if _returnvalue_2
    (Utilities|FlowControl|Sequence
      (:then_0
        (Utilities|FlowControl|DoOnce false
          (:Completed
            (bind _returnvalue_3 (Game|AddComponentbyClass (Variables|Default|GetBP%20Spectator) "/Script/Engine.StaticMeshComponent" false (Variables|Default|GetBuild%20Preview%20Transform)))
            (Variables|Default|SetPreview%20Mesh _returnvalue_3))))
      (:then_1
        (bind _output_get (Variables|Default|SetBuild%20Preview%20Transform (Math|Transform|MakeTransform (.Location (Collision|BreakHitResult _outhit)) "0, 0, 0" "1.000000,1.000000,1.000000")))
        (Transformation|SetWorldTransform (Variables|Default|GetPreview%20Mesh) _output_get false false)))))

(event EventBeginPlay
  (bind _asbp_spectator_cam (Utilities|Casting|CastToBP_SpectatorCam (Components|GetOwner)))
  (Variables|Default|SetBP%20Spectator _asbp_spectator_cam)
  (Variables|Default|SetSpectator%20Camera (Variables|/Game/Characters/BP_SpectatorCam.BP_SpectatorCam_C|GetSpectatorCamera _asbp_spectator_cam)))